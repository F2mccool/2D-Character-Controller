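; Player character for a 2D side-scrolling platformer, handling Enhanced Input movement along X, jumping and flipbook animation.
; Jumps wait for a jump-squat flipbook; releasing during it yields a short tap jump, while holding extends height up to a maximum time.
; Presses while airborne are briefly buffered and fire after the landing animation.
; Tick flips control yaw by velocity and picks airborne flipbooks, while AnimationPlaying protects jump animations from run/idle overrides.
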(event Input|EnhancedActionEvents|EnhancedInputActionIA_Jump
  (params (ActionValue :type Boolean) (ElapsedSeconds :type Float%20%28double-precision%29) (TriggeredSeconds :type Float%20%28double-precision%29) (InputAction :type Input%20Action%20Object%20Reference :default "/Game/Input/Actions/IA_Jump.IA_Jump"))
  (:Started
    (if (or (Variables|Default|GetJumping) (Variables|Default|GetFalling))
      (Variables|Default|SetJump_Buffer 0.125)
      (elif (not (Variables|Default|GetAnimation_Playing))
        (Utilities|CallJumpAnimation))))
  (:Completed
    (if (Variables|Default|GetIn_Jumpsquat)
      (Variables|Default|SetTap_Jumping true)
      (else
        (Character|StopJumping)))))

(event Input|EnhancedActionEvents|EnhancedInputActionIA_Move
  (params (ActionValue :type Float%20%28double-precision%29) (ElapsedSeconds :type Float%20%28double-precision%29) (TriggeredSeconds :type Float%20%28double-precision%29) (InputAction :type Input%20Action%20Object%20Reference :default "/Game/Input/Actions/IA_Move.IA_Move"))
  (:Triggered
    (Pawn|Input|AddMovementInput "1.000000,0.000000,0.000000" ActionValue false)
    (if (not (Variables|Default|GetAnimation_Playing))
      (Sprite|SetFlipbook (Variables|Default|GetSprite) "/Game/Paper_Assets/Character/Run_Animation/FB_Player_Run.FB_Player_Run")))
  (:Completed
    (if (not (Variables|Default|GetAnimation_Playing))
      (Sprite|SetFlipbook (Variables|Default|GetSprite) "/Game/Paper_Assets/Character/Idle_Animation/FB_Player_Idle.FB_Player_Idle"))))

(event EventBeginPlay
  (bind _asplayer_controller (Utilities|Casting|CastToPlayerController (Pawn|GetController)))
  (Input|AddMappingContext (PlayerController|LocalPlayerSubsystems|GetEnhancedInputLocalPlayerSubsystem _asplayer_controller) "/Game/Input/IMC_Platformer.IMC_Platformer" 0 "(bIgnoreAllPressedKeysUntilRelease=True,bForceImmediately=False,bNotifyUserSettings=False)"))

(event EventTick
  (params (DeltaSeconds :type Float%20%28single-precision%29))
  (bind (_x_velocity _y_velocity) (CallFunction|FindXandYVelocity))
  (Variables|Default|SetX_Velocity _x_velocity)
  (Variables|Default|SetY_Velocity _y_velocity)
  (CallFunction|SetPlayerDirection (Variables|Default|GetX_Velocity) (Pawn|GetController))
  (if (or (Variables|Default|GetJumping) (Variables|Default|GetFalling))
    (CallFunction|SetAirborneAnimation (Variables|Default|GetY_Velocity))
    (Variables|Default|SetJump_Buffer (- (Variables|Default|GetJump_Buffer) (Utilities|Time|GetWorldDeltaSeconds)))))

(event EventOnWalkingOffLedge
  (params (PreviousFloorImpactNormal :type Vector%20%28by%20ref%29 :default "0, 0, 0") (PreviousFloorContactNormal :type Vector%20%28by%20ref%29 :default "0, 0, 0") (PreviousLocation :type Vector%20%28by%20ref%29 :default "0, 0, 0") (TimeDelta :type Float%20%28single-precision%29))
  (Sprite|SetFlipbook (Variables|Default|GetSprite) "/Game/Paper_Assets/Character/Airborne_Animations/Falling/FB_Falling.FB_Falling")
  (Variables|Default|SetFalling true))

(event EventOnJumped
  (Sprite|SetFlipbook (Variables|Default|GetSprite) "/Game/Paper_Assets/Character/Airborne_Animations/Rising/FB_Rising.FB_Rising")
  (Variables|Default|SetJumping true)
  (Variables|Default|SetAnimation_Playing true)
  (Variables|Default|SetIn_Jumpsquat false))

(event EventOnLanded
  (params (Hit :type Hit%20Result%20Structure%20%28by%20ref%29))
  (Sprite|SetFlipbook (Variables|Default|GetSprite) "/Game/Paper_Assets/Character/Airborne_Animations/Landing/FB_Landing.FB_Landing")
  (Variables|Default|SetAnimation_Playing true)
  (Variables|Default|SetJumping false)
  (Variables|Default|SetFalling false)
  (Utilities|FlowControl|Delay (Class|PaperFlipbookComponent|GetFlipbookLength (Variables|Default|GetSprite)))
  (if (> (Variables|Default|GetJump_Buffer) 0.0)
    (if (Input|EnhancedActionValues|GetIA_Jump)
      _
      (else
        (Variables|Default|SetTap_Jumping true)))
    (Utilities|CallJumpAnimation)
    (else
      (CallFunction|FindAnimationtoPlaywhenLanded (Input|EnhancedActionValues|GetIA_Move)))))

(fn ConstructionScript
  (Variables|Default|SetJumpMaxHoldTime (Variables|Default|GetMaximum_Jump_Time)))

(fn SetPlayerDirection
  (params (X_Velocity :type Float%20%28double-precision%29) (Target_Controller :type Controller%20Object%20Reference))
  (if (> X_Velocity 0.0)
    (Pawn|SetControlRotation Target_Controller (Math|Rotator|MakeRotator 0.0 0.0 0.0))
    (elif (< X_Velocity 0.0)
      (Pawn|SetControlRotation Target_Controller (Math|Rotator|MakeRotator 0.0 0.0 1.8e+02))))
  (return))

(fn FindXandYVelocity
  (bind _returnvalue (Transformation|GetVelocity))
  (bind (_x _y _z) (Math|Vector|BreakVector _returnvalue))
  (return _x _z))

(fn SetAirborneAnimation
  (params (Y_Velocity :type Float%20%28double-precision%29))
  (if (> Y_Velocity 2.5e+02)
    (Sprite|SetFlipbook (Variables|Default|GetSprite) "/Game/Paper_Assets/Character/Airborne_Animations/Rising/FB_Rising.FB_Rising")
    (elif (< Y_Velocity -2.5e+02)
      (Sprite|SetFlipbook (Variables|Default|GetSprite) "/Game/Paper_Assets/Character/Airborne_Animations/Hang_Time/FB_Hang_Time.FB_Hang_Time")
      (else
        (Sprite|SetFlipbook (Variables|Default|GetSprite) "/Game/Paper_Assets/Character/Airborne_Animations/Falling/FB_Falling.FB_Falling"))))
  (return))

(fn FindAnimationtoPlaywhenLanded
  (params (Movement_Input :type Float%20%28double-precision%29))
  (Variables|Default|SetAnimation_Playing false)
  (if (> (Math|Float|Absolute(Float) Movement_Input) 0.0)
    (Sprite|SetFlipbook (Variables|Default|GetSprite) "/Game/Paper_Assets/Character/Run_Animation/FB_Player_Run.FB_Player_Run")
    (else
      (Sprite|SetFlipbook (Variables|Default|GetSprite) "/Game/Paper_Assets/Character/Idle_Animation/FB_Player_Idle.FB_Player_Idle")))
  (return))